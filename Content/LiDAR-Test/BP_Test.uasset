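; BP_Test is a LiDAR point cloud test actor with functions to find and export the points visible from a viewer camera.
; GetLidarPointCludActorsFromCamera stores visible LiDAR actors in TargetPointCloudActor, which ExportPointCloud writes to a file path with texture export on.
; Both share frustum distance, LOD radius and skip-factor settings to thin distant points.
; The event graph is empty, ResamplePointCloud calls random resampling with a zero target count, and LODExtractor is an unwired stub.
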(fn `ExportPointCloud`
  (locals (NewLocalVar :type "CameraComponent Object Reference"))
  (bind _exportfilepath_filepath (break `FilePath` (`self.exportFilePath`)))
  (`ExportVisibleLidarPointsLOD.ExportVisiblePointsLOD` (`self.targetPointCloudActor`) (`CameraActor.CameraComponent` (`self.ViewerCamera`)) _exportfilepath_filepath (`self.FrustumFar`) (`self.Near Full Res Radius`) (`self.Mid Skip Radius`) (`self.Far Skip Radius`) (`self.Skip Factor Mid`) (`self.Skip Factor Far`) true true))

(fn `GetLidarPointCludActorsFromCamera`
  (bind _returnvalue (`ExportVisibleLidarPointsLOD.GetVisibleLidarActors` (`CameraActor.CameraComponent` (`self.ViewerCamera`)) (`self.FrustumFar`) (`self.Near Full Res Radius`) (`self.Mid Skip Radius`) (`self.Far Skip Radius`) (`self.Skip Factor Mid`) (`self.Skip Factor Far`)))
  (set `self.targetPointCloudActor` _returnvalue))

(fn `LODExtractor`)

(fn `ResamplePointCloud`
  (`LidarPointCloudResampler.ResampleRandom` null))

(fn `UserConstructionScript`)