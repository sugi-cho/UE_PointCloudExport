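; Component that exports the LiDAR point clouds visible to its owner's camera to a file.
; SetPointClouds stores the LiDAR actors found within the owner's CameraComponent frustum.
; ExportPointCloud passes that stored list to a LOD export, where near, mid and far radii with skip factors control point density, with world-space and texture export options.
; Both functions are called externally, as the event graph is empty.
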(fn `ExportPointCloud`
  (bind _filepath_filepath (break `FilePath` (`self.FilePath`)))
  (`ExportVisibleLidarPointsLOD.ExportVisiblePointsLOD` (`self.PointClouds`) (`Actor.GetComponentByClass` (`self.GetOwner`) "/Script/Engine.CameraComponent") _filepath_filepath (`self.FrustumFar`) (`self.NearFullResRadius`) (`self.MidSkipRadius`) (`self.FarSkipRadius`) (`self.SkipFactorMid`) (`self.SkipFactorFar`) (`self.WorldSpace`) (`self.ExportTexture`)))

(fn `SetPointClouds`
  (bind _returnvalue (`ExportVisibleLidarPointsLOD.GetVisibleLidarActors` (`Actor.GetComponentByClass` (`self.GetOwner`) "/Script/Engine.CameraComponent") (`self.FrustumFar`) (`self.NearFullResRadius`) (`self.MidSkipRadius`) (`self.FarSkipRadius`) (`self.SkipFactorMid`) (`self.SkipFactorFar`)))
  (set `self.PointClouds` _returnvalue))